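; Player character Blueprint that links an animation class layer on BeginPlay and carries debug test hooks.
; X toggles slow motion, Z toggles a one-second loop activating abilities by tag, and C switches the mesh to physics with an impulse.
; Tick draws debug arrows for facing and last movement input.
; GetModuleName returns the Character.BP_Character_C module path; unwired test chains cover effects, launches, box traces and walk speed.
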(event `Key|X`
  (params (Key :type "Key Structure"))
  (:`Pressed`
    ;[1 1 1] Test 子弹时间
    (`/Engine/EditorBlueprintResources/StandardMacros.FlipFlop`
      (:`A`
        (`GameplayStatics.SetGlobalTimeDilation` 0.1))
      (:`B`
        (`GameplayStatics.SetGlobalTimeDilation` 1.0)))))

(event `Key|Z`
  (params (Key :type "Key Structure"))
  (:`Pressed`
    ;[1 1 1] Test 自动攻击
    (`/Engine/EditorBlueprintResources/StandardMacros.FlipFlop`
      (:`A`
        (set `self.SwitchAutoUsingSkill` true)
        (`KismetSystemLibrary.RetriggerableDelay` 1.0 :!label _label)
        (if (`self.SwitchAutoUsingSkill`)
          (`AbilitySystemComponent.TryActivateAbilitiesByTag` (`AbilitySystemBlueprintLibrary.GetAbilitySystemComponent` null) (`self.Gameplay Tag Container`) true)
          (goto _label)))
      (:`B`
        (set `self.SwitchAutoUsingSkill` false)))))

(event `self.ReceiveTick`
  (params (DeltaSeconds :type "Float (single-precision)"))
  (`|ExecutionSequence`
    (:`then_0`
      (set `self.Delta Seconds` DeltaSeconds))
    (:`then_1`
      (`self.ShowCharacterArrowByTick`))))

(event `Key|C`
  (params (Key :type "Key Structure"))
  (bind _mesh (`self.Mesh`))
  (:`Pressed`
    (`/Engine/EditorBlueprintResources/StandardMacros.FlipFlop`
      (:`A`
        _)
      (:`B`
        _))
    (`PrimitiveComponent.SetSimulatePhysics` _mesh true)
    (`PrimitiveComponent.SetEnableGravity` _mesh true)
    (`PrimitiveComponent.SetCollisionEnabled` _mesh "PhysicsOnly")
    (`PrimitiveComponent.SetCollisionResponseToChannel` _mesh "ECC_WorldStatic" "ECR_Block")
    (`PrimitiveComponent.AddImpulse` _mesh (20000.0 20000.0 100.0) "None" false)))

(event `self.ReceiveBeginPlay`
  (`SkeletalMeshComponent.LinkAnimClassLayers` (`self.Mesh`) (`self.LinkedAnimClassLayer`)))

(fn `GetModuleName`
  (returns (ReturnValue :type String))
  (return "Character.BP_Character_C"))

(fn `ShowCharacterArrowByTick`
  (bind _returnvalue (+ (`self.K2_GetActorLocation`) (0.0 0.0 -40.0)))
  (bind _returnvalue_2 (+ (`self.K2_GetActorLocation`) (0.0 0.0 -50.0)))
  (`KismetSystemLibrary.DrawDebugArrow` _returnvalue_2 (+ _returnvalue_2 (* (`self.GetActorForwardVector`) (200.0 200.0 200.0))) 50.0 (struct :`G` 0.139122 :`B` 1.0 :`A` 1.0) (* (`self.Delta Seconds`) 1.1) 5.0)
  (`KismetSystemLibrary.DrawDebugArrow` _returnvalue (+ _returnvalue (* (`self.GetLastMovementInputVector`) (200.0 200.0 200.0))) 50.0 (struct :`G` 1.0 :`B` 0.811846 :`A` 1.0) (* (`self.Delta Seconds`) 1.1) 5.0))

(fn `UserConstructionScript`)