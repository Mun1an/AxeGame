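; Light hit-reaction gameplay ability that plays a directional montage when a character is hit.
; On authority it plays the reaction and, for characters not locally controlled, passes the hit result to OnHitResult, which stores it and enters the same montage path.
; The hit direction selects the opposite-named front, back, left or right montage.
; A notify-state task accompanies the montage, and completion, interruption or cancellation ends the ability.
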(event `self.K2_ActivateAbility`
  (`self.K2_HasAuthority`
    (:`True`
      (`self.IsLocallyControlled`
        (:`True`
          _)
        (:`False`
          (`self.OnHitResult` (`self.HitResult`))))
      (`|ExecutionSequence` :!label _label
        (:`then_0`
          (set `self.AbilityMontage` (select `ELaunchCharacterDirection` (`self.GetHitDirectionMontageByHitResult` (`self.HitResult`)) :`Lc_Forward` (`self.HitReactMontage_B`) :`Lc_Backward` (`self.HitReactMontage_F`) :`Lc_Left` (`self.HitReactMontage_R`) :`Lc_Right` (`self.HitReactMontage_L`))))
        (:`then_1`
          (`AbilityTask_PlayMontageAndWait.CreatePlayMontageAndWaitProxy` "None" (`self.AbilityMontage`) 1.0 "None" false
            (:`then`
              (`self.AddMontageNotifyStateTask` (`self.AbilityMontage`)))
            (:`OnCompleted`
              (`self.K2_EndAbility` :!label _label_2))
            (:`OnInterrupted`
              (goto _label_2))
            (:`OnCancelled`
              (goto _label_2))))))))

(event `OnHitResult`
  (params (NewHitResult :type "HitResult Structure"))
  (set `self.HitResult` NewHitResult)
  (goto _label))