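; Player shield parry gameplay ability for the axe-and-shield defense set.
; On activation it plays the ability montage with a montage notify-state task and ends when the montage completes, is interrupted or is cancelled.
; It also adds the ShieldParry gameplay cue at the owner's location, removed on ability end, and shakes the camera.
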(event `self.K2_ActivateAbility`
  (bind _returnvalue (`Actor.K2_GetActorLocation` (`self.GetAxeCharacterOwner`)))
  (`|ExecutionSequence`
    (:`then_0`
      (`AbilityTask_PlayMontageAndWait.CreatePlayMontageAndWaitProxy` "None" (`self.AbilityMontage`)
        (:`then`
          (`self.AddMontageNotifyStateTask` (`self.AbilityMontage`)))
        (:`OnCompleted`
          (`self.K2_EndAbility` :!label _label))
        (:`OnInterrupted`
          (goto _label))
        (:`OnCancelled`
          (goto _label))))
    (:`then_1`
      (`self.K2_AddGameplayCueWithParams` (struct :`TagName` "GameplayCue.ShieldParry") (`AbilitySystemBlueprintLibrary.MakeGameplayCueParameters` 0.0 0.0 (struct) (struct) (struct) (struct) (struct) _returnvalue _returnvalue)))
    (:`then_2`
      (`self.ShakeCamera`))))