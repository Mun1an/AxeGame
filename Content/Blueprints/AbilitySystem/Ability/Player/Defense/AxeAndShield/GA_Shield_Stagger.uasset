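; GA_Shield_Stagger is a player Gameplay Ability for the axe-and-shield defense set that plays a stagger reaction.
; On activation it plays the ability montage at half speed, starts a montage notify-state task alongside it, and shakes the camera.
; The ability ends when the montage completes, is interrupted or is cancelled.
; A ShieldParry gameplay cue at the owner's location is present but unconnected, so it never fires.
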(event `self.K2_ActivateAbility`
  (`|ExecutionSequence`
    (:`then_0`
      (`AbilityTask_PlayMontageAndWait.CreatePlayMontageAndWaitProxy` "None" (`self.AbilityMontage`) 0.5
        (:`then`
          (`self.AddMontageNotifyStateTask` (`self.AbilityMontage`)))
        (:`OnCompleted`
          (`self.K2_EndAbility` :!label _label))
        (:`OnInterrupted`
          (goto _label))
        (:`OnCancelled`
          (goto _label))))
    (:`then_2`
      (`self.ShakeCamera`))))