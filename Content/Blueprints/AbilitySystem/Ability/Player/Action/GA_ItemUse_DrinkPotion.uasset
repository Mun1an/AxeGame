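; Player gameplay ability for drinking a potion item.
; On activation it plays the drink montage at a faster rate and commits the ability when a "Commit" montage notify fires, ending when the montage completes or is interrupted.
; The server spawns a display item actor on the secondary hand socket, replacing any previous one, and destroys it when the ability ends.
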(event `self.BP_OnCustomNameNotifyBegin`
  (params (CustomName :type Name))
  (switch `name` CustomName
    (:`Commit`
      (`self.K2_CommitAbility`))))

(event `self.K2_ActivateAbility`
  (`|ExecutionSequence` :!label _label
    (:`then_0`
      (`AbilityTask_PlayMontageAndWait.CreatePlayMontageAndWaitProxy` "None" (`self.AbilityMontage`) 1.5
        (:`then`
          (`self.AddMontageNotifyStateTask` (`self.AbilityMontage`)))
        (:`OnCompleted`
          (`self.K2_EndAbility` :!label _label_2))
        (:`OnInterrupted`
          (goto _label_2))
        (:`OnCancelled`
          (goto _label_2))))
    (:`then_1`
      (`self.K2_HasAuthority`
        (:`True`
          (`|ExecutionSequence`
            (:`then_0`
              (`/Engine/EditorBlueprintResources/StandardMacros.IsValid` (`self.DisplayItemActor`)
                (:`Is Valid`
                  (`Actor.K2_DestroyActor` (`self.DisplayItemActor`))
                  (set `self.DisplayItemActor` null))))
            (:`then_1`
              (bind _returnvalue (`self.CreateItemDisplayActor` (`Actor.GetTransform` (`self.GetAxeCharacterOwner`)) "WeaponSecondaryHandSocket"))
              (set `self.DisplayItemActor` _returnvalue))))))))

(event `self.K2_ActivateAbilityFromEvent`
  (params (EventData :type "GameplayEventData Structure (by ref)"))
  (goto _label))

(event `self.K2_OnEndAbility`
  (params (bWasCancelled :type Boolean))
  (`self.K2_HasAuthority`
    (:`True`
      (`/Engine/EditorBlueprintResources/StandardMacros.IsValid` (`self.DisplayItemActor`)
        (:`Is Valid`
          (`Actor.K2_DestroyActor` (`self.DisplayItemActor`))
          (set `self.DisplayItemActor` null))))))