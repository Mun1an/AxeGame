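; Gameplay ability that collects a pickup into the player's inventory when triggered by a gameplay event.
; It reads the item instance and count from the event target as a Pickupable, then adds them to the instigating AxeCharacterPlayer's InventoryComponent.
; After the add call it destroys the target without checking the result.
; The ability ends through a final sequence step, or immediately if the target is invalid.
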(event `self.K2_ActivateAbility`)

(event `self.K2_ActivateAbilityFromEvent`
  (params (EventData :type "GameplayEventData Structure (by ref)"))
  (bind (_eventtag _instigator _target) (break `GameplayEventData` EventData))
  (`/Engine/EditorBlueprintResources/StandardMacros.IsValid` _target
    (:`Is Valid`
      (`|ExecutionSequence`
        (:`then_1`
          (bind _aspickupable (cast `Pickupable` _target))
          (bind _returnvalue (`Pickupable.GetPickupableItemInstance` _aspickupable))
          (bind _returnvalue_2 (`Pickupable.GetPickupableItemCount` _aspickupable)))
        (:`then_2`
          (bind _asaxe_character_player (cast `AxeCharacterPlayer` _instigator))
          (`InventoryComponent.AddItemInstance` (`AxeCharacterPlayer.InventoryComponent` _asaxe_character_player) _returnvalue _returnvalue_2 -1)
          (`/Engine/EditorBlueprintResources/StandardMacros.IsValid` _target
            (:`Is Valid`
              (`Actor.K2_DestroyActor` _target))))
        (:`then_3`
          (`self.K2_EndAbility` :!label _label))))
    (:`Is Not Valid`
      (goto _label))))