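; GA_Interact_Talk is the player's interact ability for talking to a shop NPC, opening that NPC's shop UI.
; When triggered by an event on the locally controlled client, it casts the event target to BP_ShopNPC and creates a WBP_Shop bound to its ShopComponent.
; The widget goes through AxeUIManagerSubsystem, then the ability ends; non-local or invalid-target activations end immediately.
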(event `self.K2_ActivateAbility`)

(event `self.K2_ActivateAbilityFromEvent`
  (params (EventData :type "GameplayEventData Structure (by ref)"))
  (bind (_eventtag _instigator _target) (break `GameplayEventData` EventData))
  (`self.IsLocallyControlled`
    (:`True`
      (`/Engine/EditorBlueprintResources/StandardMacros.IsValid` _target
        (:`Is Valid`
          (`|ExecutionSequence`
            (:`then_0`
              (bind _asbp_shop_npc (cast `/Game/Blueprints/Character/Mob/NPC/BP_ShopNPC` _target))
              (bind _returnvalue (`|CreateWidget` "/Game/Blueprints/UI/Shop/WBP_Shop.WBP_Shop_C" null (`/Game/Blueprints/Character/Mob/NPC/BP_ShopNPC.ShopComponent` _asbp_shop_npc)))
              (`AxeUIManagerSubsystem.AddUIWidget` (subsystem `AxeUIManagerSubsystem`) _returnvalue))
            (:`then_3`
              (`self.K2_EndAbility`))))
        (:`Is Not Valid`
          (`self.K2_EndAbility` :!label _label))))
    (:`False`
      (goto _label))))