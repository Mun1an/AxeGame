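; Player skill Gameplay Ability that throws an axe projectile toward a target location.
; On activation it calls commit, plays the ability montage with a notify-state task, and ends when the montage completes, is interrupted or is cancelled.
; The montage's "Throw Axe" custom notify times the throw, spawning the projectile only with authority, at the character's location and rotated along the target direction.
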(event `self.K2_ActivateAbility`
  (`|ExecutionSequence`
    (:`then_0`
      (`self.K2_CommitAbility`))
    (:`then_1`
      (`AbilityTask_PlayMontageAndWait.CreatePlayMontageAndWaitProxy` "None" (`self.AbilityMontage`)
        (:`then`
          (`self.AddMontageNotifyStateTask` (`self.AbilityMontage`)))
        (:`OnCompleted`
          (`self.K2_EndAbility` :!label _label))
        (:`OnInterrupted`
          (goto _label))
        (:`OnCancelled`
          (goto _label))))))

(event `self.BP_OnCustomNameNotifyBegin`
  (params (CustomName :type Name))
  (switch `name` CustomName
    (:`ThrowAxe`
      (`self.K2_HasAuthority`
        (:`True`
          (bind _returnvalue (`self.GetDirectionByTargetLocation`))
          (`self.SpawnProjectile` (`KismetMathLibrary.MakeTransform` (`Actor.K2_GetActorLocation` (`self.GetAxeCharacterOwner`)) (`KismetMathLibrary.Conv_VectorToRotator` _returnvalue))))))))