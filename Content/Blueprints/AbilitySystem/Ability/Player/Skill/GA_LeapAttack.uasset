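; Player leap attack ability that jumps forward and smashes the ground, damaging enemies in a radius on landing.
; Activation commits and plays a montage, whose Jump notify starts a root-motion jump force using computed direction and auto-target distance.
; Finish or landing, guarded to fire once, runs an authority-only sphere overlap for damage and adds a GroundSmash cue at the ground point below.
; The ability ends when the montage completes or is interrupted or cancelled.
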(event `self.K2_ActivateAbility`
  (`|ExecutionSequence`
    (:`then_0`
      (`self.K2_CommitAbility`)
      (`AbilityTask_PlayMontageAndWait.CreatePlayMontageAndWaitProxy` "None" (`self.AbilityMontage`)
        (:`then`
          (`self.AddMontageNotifyStateTask` (`self.AbilityMontage`)))
        (:`OnCompleted`
          (`self.K2_EndAbility` :!label _label))
        (:`OnInterrupted`
          (goto _label))
        (:`OnCancelled`
          (goto _label))))))

(event `self.BP_OnCustomNameNotifyBegin`
  (params (CustomName :type Name))
  (bind _returnvalue (`self.GetAxeCharacterOwner`))
  (switch `name` CustomName
    (:`Jump`
      (`|ExecutionSequence`
        (:`then_0`
          (set `self.IsStartDamage` false))
        (:`then_1`
          (bind _returnvalue_2 (`self.GetJumpDistanceByAutoTarget`))
          (bind _returnvalue_3 (`self.GetJumpDirection`)))
        (:`then_2`
          (`AbilityTask_ApplyRootMotionJumpForce.ApplyRootMotionJumpForce` "None" (`KismetMathLibrary.Conv_VectorToRotator` _returnvalue_3) _returnvalue_2 (`self.JumpHeight`) (`self.JumpDuration`) 0.0 true "ClampVelocity" (0.0 0.0 0.0) 100.0
            (:`OnFinish`
              _)
            (:`OnLanded`
              _))
          (if (not (`self.IsStartDamage`))
            (set `self.IsStartDamage` true)
            (`|ExecutionSequence`
              (:`then_0`
                ;[1 1 1] AreaDamage
                (`self.K2_HasAuthority`
                  (:`True`
                    (bind _outactors (`KismetSystemLibrary.SphereOverlapActors` (`Actor.K2_GetActorLocation` (`self.GetAxeCharacterOwner`)) (`self.Damage Sphere Radius`) (`self.Object Types`) "/Script/Axe.AxeCharacterEnemy" (`self.Ignore Actors`)))
                    (for _array_element _outactors
                      (bind _asaxe_character_base (cast `AxeCharacterBase` _array_element))
                      (`self.ApplyDamageToTarget` _asaxe_character_base (`GameplayStatics.MakeHitResult` false))))))
              (:`then_1`
                ;[1 1 1] Particle
                (bind _returnvalue_4 (`AxeBlueprintFunctionLibrary.GetBottomGroundLocation` _returnvalue (`Actor.K2_GetActorLocation` _returnvalue)))
                (`self.K2_AddGameplayCueWithParams` (struct :`TagName` "GameplayCue.GroundSmash") (`AbilitySystemBlueprintLibrary.MakeGameplayCueParameters` 0.0 0.0 (struct) (struct) (struct) (struct) (struct) _returnvalue_4))))))))))