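; Gameplay ability that makes the player character dash along its last movement input, defaulting to backward when there is none.
; After committing, it selects a forward, back, left or right montage from that direction and adds a notify-state task for it.
; An additive root motion constant force with gravity drives the movement and clamps exit velocity.
; The ability ends when the montage completes or breaks off, or if commit fails.
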(event `self.K2_ActivateAbility`
  (`|ExecutionSequence`
    (:`then_0`
      (set `self.LastMovementInput` (* (`Actor.GetActorForwardVector` (`self.GetAxeCharacterOwner`)) (-1.0 -1.0 -1.0))))
    (:`then_1`
      (bind _asaxe_character_player (cast `AxeCharacterPlayer` (`self.GetAxeCharacterOwner`)))
      (bind (_asynctaskproxy _lastmoveinput) (`AbilityTask_WaitLastMoveInput.CreateWaitLastMoveInputTask` _asaxe_character_player)
        (:`OnLastMoveInputDelegate`
          (if (not (`KismetMathLibrary.Vector_IsNearlyZero` _lastmoveinput 0.001))
            (set `self.LastMovementInput` _lastmoveinput))
          (bind _returnvalue (`self.K2_CommitAbility`))
          (if _returnvalue
            (`|ExecutionSequence`
              (:`then_0`
                (set `self.AbilityMontage` (select `ELaunchCharacterDirection` (`self.GetDashDirectionByMovementVector` (`self.LastMovementInput`)) :`Lc_Forward` (`self.DashMontage_F`) :`Lc_Backward` (`self.DashMontage_B`) :`Lc_Left` (`self.DashMontage_L`) :`Lc_Right` (`self.DashMontage_R`))))
              (:`then_1`
                (`AbilityTask_PlayMontageAndWait.CreatePlayMontageAndWaitProxy` "None" (`self.AbilityMontage`) 1.0 "None" false
                  (:`then`
                    (`self.AddMontageNotifyStateTask` (`self.AbilityMontage`)))
                  (:`OnCompleted`
                    (`self.K2_EndAbility` :!label _label))
                  (:`OnInterrupted`
                    (goto _label))
                  (:`OnCancelled`
                    (goto _label))))
              (:`then_2`
                (`AbilityTask_ApplyRootMotionConstantForce.ApplyRootMotionConstantForce` "None" (`self.LastMovementInput`) (`self.DashStrength`) (`self.DashDuration`) true null "ClampVelocity" (0.0 0.0 0.0) 500.0 true)))
            (else
              (`self.K2_EndAbility`))))))))