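; Gameplay ability for the wolf mob's melee attack.
; On activation it plays the ability montage, listens for its notify states and ends when the montage completes, is interrupted or is cancelled.
; A "Light Attack" notify runs a sphere overlap at the mesh's AttackSlot socket, ignoring the wolf, and applies damage to each overlapped non-friendly AxeCharacterBase.
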(event `self.K2_ActivateAbility`
  (`AbilityTask_PlayMontageAndWait.CreatePlayMontageAndWaitProxy` "None" (`self.AbilityMontage`)
    (:`then`
      (`self.AddMontageNotifyStateTask` (`self.AbilityMontage`)))
    (:`OnCompleted`
      (`self.K2_EndAbility` :!label _label))
    (:`OnInterrupted`
      (goto _label))
    (:`OnCancelled`
      (goto _label))))

(event `self.BP_OnCustomNameNotifyBegin`
  (params (CustomName :type Name))
  (switch `name` CustomName
    (:`LightAttack`
      (`|ExecutionSequence`
        (:`then_0`
          (`KismetArrayLibrary.Array_Clear` (`self.Actors to Ignore`)))
        (:`then_1`
          (`KismetArrayLibrary.Array_AddUnique` (`self.Actors to Ignore`) (`self.GetAxeCharacterOwner`))
          (bind _outactors (`KismetSystemLibrary.SphereOverlapActors` (`SceneComponent.GetSocketLocation` (`Character.Mesh` (`self.GetAxeCharacterOwner`)) "AttackSlot") 50.0 (`self.Object Types`) null (`self.Actors to Ignore`)))
          (for _array_element _outactors
            (if (not (`AxeBlueprintFunctionLibrary.IsFriend` _array_element (`self.GetAxeCharacterOwner`)))
              (bind _asaxe_character_base (cast `AxeCharacterBase` _array_element))
              (`self.ApplyDamageToTarget` _asaxe_character_base (`GameplayStatics.MakeHitResult` false)))))))))