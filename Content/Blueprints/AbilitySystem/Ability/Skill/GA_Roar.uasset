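; GA_Roar is a Gameplay Ability for a roar skill that buffs or otherwise affects its owner through a gameplay effect.
; On activation it commits, plays the ability montage with a notify-state task, and ends when the montage completes, is interrupted or is cancelled.
; In the same activation it builds an outgoing effect spec, overrides its duration with EffectDuration, and applies it to the owner without waiting for the montage.
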(event `self.K2_ActivateAbility`
  (`|ExecutionSequence`
    (:`then_0`
      (`self.K2_CommitAbility`))
    (:`then_1`
      (`AbilityTask_PlayMontageAndWait.CreatePlayMontageAndWaitProxy` "None" (`self.AbilityMontage`)
        (:`then`
          (`self.AddMontageNotifyStateTask` (`self.AbilityMontage`)))
        (:`OnCompleted`
          (`self.K2_EndAbility` :!label _label))
        (:`OnInterrupted`
          (goto _label))
        (:`OnCancelled`
          (goto _label))))
    (:`then_2`
      (bind _returnvalue (`AbilitySystemBlueprintLibrary.SetDuration` (`self.MakeOutgoingGameplayEffectSpec` (`self.Gameplay Effect Class`)) (`self.Effect Duration`)))
      (`self.K2_ApplyGameplayEffectSpecToOwner` _returnvalue))))