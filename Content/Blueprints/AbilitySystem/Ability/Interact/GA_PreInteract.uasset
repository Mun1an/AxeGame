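; GA_PreInteract is a gameplay ability that highlights the current interactable target and triggers interaction on input.
; On activation it waits for an input press, then calls TriggerInteraction and ends itself.
; When the target changes on the locally controlled client, it casts to HighLight to unhighlight the previous target and highlight the new one.
; LastHighLightTarget tracks the highlighted actor; the OnEndAbility event is unused, so it clears no highlight.
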(event `self.K2_ActivateAbility`
  (`AbilityTask_WaitInputPress.WaitInputPress` false
    (:`OnPress`
      (`self.TriggerInteraction`)
      (`self.K2_EndAbility`))))

(event `self.OnTargetInteractableChange`
  (`self.IsLocallyControlled`
    (:`True`
      (`|ExecutionSequence`
        (:`then_0`
          (`/Engine/EditorBlueprintResources/StandardMacros.IsValid` (`self.LastHighLightTarget`)
            (:`Is Valid`
              (if (!= (`self.LastHighLightTarget`) (`self.CurrentTarget`))
                (bind _ashigh_light (cast `HighLight` (`self.LastHighLightTarget`)))
                (`HighLight.UnHighlightActor` _ashigh_light)))))
        (:`then_1`
          (`/Engine/EditorBlueprintResources/StandardMacros.IsValid` (`self.CurrentTarget`)
            (:`Is Valid`
              (bind _ashigh_light_2 (cast `HighLight` (`self.CurrentTarget`)))
              (`HighLight.HighlightActor` _ashigh_light_2)
              (set `self.LastHighLightTarget` (`self.CurrentTarget`)))))))))